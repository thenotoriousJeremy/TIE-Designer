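; BP_Piece is an editable building piece, apparently for assembling fighters, that the player selects, places and transforms with mouse and keys.
; BeginPlay swaps mesh materials by slot name for dynamic ones from TIEPlayerController.
; Clicks toggle selection, which clears other pieces' input and enables this one's; while selected, Tick snaps it to a grid under the cursor with an outline overlay.
; Input actions delete, scale, mirror, and either rotate or nudge, depending on Caps Lock.
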(event Custom|NotFocus
  (Input|DisableInput (Game|GetPlayerController 0))
  (Variables|Default|SetCurrent false)
  (Rendering|Material|SetOverlayMaterial (Variables|Default|GetStaticMesh) 0 :!class /Script/Engine.MeshComponent))

(event EventBeginPlay
  (Input|EnableInput (Game|GetPlayerController 0))
  (Utilities|FlowControl|RetriggerableDelay 0.2)
  (bind _staticmesh (Variables|Default|GetStaticMesh)
    (:then
      (Development|PrintString (Utilities|String|ToString(Integer) (Rendering|Material|GetNumMaterials _staticmesh)))
      (bind _astieplayer_controller (Utilities|Casting|CastToTIEPlayerController (Game|GetPlayerController 0)))
      (for _array_element (Class|PrimitiveComponent|GetMaterialSlotNames _staticmesh)
        (Development|PrintString (Utilities|String|ToString(Name) _array_element))
        (Rendering|Material|SetMaterialbyName (Variables|Default|GetStaticMesh) _array_element (Utilities|Array|Get(acopy) (Variables|/Game/Blueprints/TIEPlayerController.TIEPlayerController_C|GetMaterialsDynamic _astieplayer_controller) (Utilities|Array|FindItem (Variables|Default|GetMaterialList) _array_element)))))
    (:else)))

(event Collision|EventActorBeginOverlap
  (params (OtherActor :type Actor%20Object%20Reference)))

(event EventTick
  (params (DeltaSeconds :type Float%20%28single-precision%29))
  (bind _returnvalue (Game|GetPlayerController 0))
  (bind (_worldlocation _worlddirection) (Game|Player|ConvertMouseLocationToWorldSpace _returnvalue))
  (if (Variables|Default|GetCurrent)
    (bind (_outhit _returnvalue_2) (Collision|LineTraceByChannel _worldlocation (+ _worldlocation (* _worlddirection 1e+04)) "TraceTypeQuery1" false 0 "ForDuration"))
    (if _returnvalue_2
      (Transformation|SetActorLocation self (Math|Vector|MakeVector (Math|Conversions|ToFloat(Integer) (* (Math|Float|Round (/ (.X (Math|Vector|BreakVector (.location _outhit))) 5e+01)) 50)) (Math|Conversions|ToFloat(Integer) (* (Math|Float|Round (/ (.Y (Math|Vector|BreakVector (.location _outhit))) 5e+01)) 50)) (Math|Conversions|ToFloat(Integer) (* (Math|Float|Round (/ (.Z (Math|Vector|BreakVector (.location _outhit))) 5e+01)) 50))) false false)
      (Rendering|Material|SetOverlayMaterial (Variables|Default|GetStaticMesh) "/Game/Fighters/M_Outline.M_Outline" :!class /Script/Engine.MeshComponent))))

(event MouseInput|EventActorOnClicked
  (params (ButtonPressed :type Key%20Structure :default "None"))
  (bind _returnvalue (Game|GetPlayerController 0))
  (bind _staticmesh (Variables|Default|GetStaticMesh))
  (if (not (Variables|Default|GetFirst))
    (Utilities|FlowControl|FlipFlop
      (:A
        (Input|DisableInput _returnvalue)
        (Variables|Default|SetCurrent false)
        (Rendering|Material|SetOverlayMaterial _staticmesh 0 :!class /Script/Engine.MeshComponent))
      (:B
        (bind _outactors (Actor|GetAllActorsOfClass "BP_Piece_C"))
        (for _array_element _outactors
          (Variables|BP_Piece_C|SetCurrent _array_element false)
          (Input|DisableInput _array_element _returnvalue))
        (Input|EnableInput _returnvalue)
        (Variables|Default|SetCurrent true)
        (Rendering|Material|SetOverlayMaterial _staticmesh "/Game/Fighters/M_Outline.M_Outline" :!class /Script/Engine.MeshComponent)))))

(event Input|ActionEvents|InputActionScale-
  (params (Key :type Key%20Structure :default "None"))
  (:Pressed
    (Transformation|SetActorScale3D (* (Transformation|GetActorScale3D self) 0.75))))

(event Input|ActionEvents|InputActionMirror
  (params (Key :type Key%20Structure :default "None"))
  (bind _defaultsceneroot (Variables|Default|GetDefaultSceneRoot))
  (bind _returnvalue (Transformation|GetWorldScale _defaultsceneroot))
  (:Pressed
    (Transformation|SetWorldScale3D _defaultsceneroot (Math|Vector|MakeVector (* (.x _returnvalue) -1.0) (.y _returnvalue) (.z _returnvalue)))))

(event Input|ActionEvents|InputActionDelete
  (params (Key :type Key%20Structure :default "None"))
  (:Pressed
    (Actor|DestroyActor)))

(event Input|ActionEvents|InputActionPitch+
  (params (Key :type Key%20Structure :default "None"))
  (:Pressed
    (Variables|Default|SetDirection 1.0)
    (if (Class|MyBlueprintFunctionLibrary|AreCapsLocked)
      (Class|Actor|AddActorWorldRotation (Math|Rotator|MakeRotator 0.0 (* (Variables|Default|GetDirection) 15.0) 0.0))
      (else
        (Transformation|AddLocalOffset (Variables|Default|GetStaticMesh) (Math|Vector|MakeVector (* (Variables|Default|GetDirection) 1e+01) 0.0 0.0) false false)))))

(event Input|ActionEvents|InputActionPitch-
  (params (Key :type Key%20Structure :default "None"))
  (:Pressed
    (Variables|Default|SetDirection -1.0)
    (if (Class|MyBlueprintFunctionLibrary|AreCapsLocked)
      (Class|Actor|AddActorWorldRotation (Math|Rotator|MakeRotator 0.0 (* (Variables|Default|GetDirection) 15.0) 0.0))
      (else
        (Transformation|AddLocalOffset (Variables|Default|GetStaticMesh) (Math|Vector|MakeVector (* (Variables|Default|GetDirection) 1e+01) 0.0 0.0) false false)))))

(event Input|ActionEvents|InputActionRoll+
  (params (Key :type Key%20Structure :default "None"))
  (:Pressed
    (Variables|Default|SetDirection 1.0)
    (if (Class|MyBlueprintFunctionLibrary|AreCapsLocked)
      (Class|Actor|AddActorWorldRotation (Math|Rotator|MakeRotator (* (Variables|Default|GetDirection) 15.0) 0.0 0.0))
      (else
        (Transformation|AddLocalOffset (Variables|Default|GetStaticMesh) (Math|Vector|MakeVector 0.0 (* (Variables|Default|GetDirection) 1e+01) 0.0) false false)))))

(event Input|ActionEvents|InputActionRoll-
  (params (Key :type Key%20Structure :default "None"))
  (:Pressed
    (Variables|Default|SetDirection -1.0)
    (if (Class|MyBlueprintFunctionLibrary|AreCapsLocked)
      (Class|Actor|AddActorWorldRotation (Math|Rotator|MakeRotator (* (Variables|Default|GetDirection) 15.0) 0.0 0.0))
      (else
        (Transformation|AddLocalOffset (Variables|Default|GetStaticMesh) (Math|Vector|MakeVector 0.0 (* (Variables|Default|GetDirection) 1e+01) 0.0) false false)))))

(event Input|ActionEvents|InputActionYaw+
  (params (Key :type Key%20Structure :default "None"))
  (:Pressed
    (Variables|Default|SetDirection 1.0)
    (if (Class|MyBlueprintFunctionLibrary|AreCapsLocked)
      (Class|Actor|AddActorWorldRotation (Math|Rotator|MakeRotator 0.0 0.0 (* (Variables|Default|GetDirection) 15.0)))
      (else
        (Transformation|AddLocalOffset (Variables|Default|GetStaticMesh) (Math|Vector|MakeVector 0.0 0.0 (* (Variables|Default|GetDirection) 1e+01)) false false)))))

(event Input|ActionEvents|InputActionYaw-
  (params (Key :type Key%20Structure :default "None"))
  (:Pressed
    (Variables|Default|SetDirection -1.0)
    (if (Class|MyBlueprintFunctionLibrary|AreCapsLocked)
      (Class|Actor|AddActorWorldRotation (Math|Rotator|MakeRotator 0.0 0.0 (* (Variables|Default|GetDirection) 15.0)))
      (else
        (Transformation|AddLocalOffset (Variables|Default|GetStaticMesh) (Math|Vector|MakeVector 0.0 0.0 (* (Variables|Default|GetDirection) 1e+01)) false false)))))

(event Input|ActionEvents|InputActionScale+
  (params (Key :type Key%20Structure :default "None"))
  (:Pressed
    (Transformation|SetActorScale3D (* (Transformation|GetActorScale3D self) 1.333333))))

(fn ConstructionScript)