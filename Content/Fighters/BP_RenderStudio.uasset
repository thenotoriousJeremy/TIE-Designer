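; BP_RenderStudio is a single-use actor that renders a given static mesh into a render target exposed through a dynamic material.
; Capture adds the mesh, offsets the SceneCaptureComponent2D diagonally by its bounds radius and aims it at the bounds origin.
; The capture shows only this actor and feeds a new render target into an M_Render instance stored in Render.
; After a short delay it captures once, then destroys itself.
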(event Custom|Capture
  (params (StaticMesh :type Static%20Mesh%20Object%20Reference))
  (bind _scenecapturecomponent2d (Variables|Default|GetSceneCaptureComponent2D))
  (bind _scenecapturecomponent2d_2 (Variables|Default|GetSceneCaptureComponent2D))
  (bind _returnvalue (AddComponent|AddStaticMeshComponent false))
  (Components|StaticMesh|SetStaticMesh _returnvalue StaticMesh)
  (Transformation|SetRelativeLocation _scenecapturecomponent2d (Math|Vector|MakeVector (* (.SphereRadius (Collision|GetComponentBounds _returnvalue)) 1.0) (* (.SphereRadius (Collision|GetComponentBounds _returnvalue)) 1.0) (* (.SphereRadius (Collision|GetComponentBounds _returnvalue)) 1.0)) false false)
  (Transformation|SetWorldRotation _scenecapturecomponent2d (Math|Rotator|FindLookatRotation (Transformation|GetWorldLocation _scenecapturecomponent2d) (.Origin (Collision|GetComponentBounds _returnvalue))) false false)
  (bind _returnvalue_2 (Rendering|CreateRenderTarget2D 256 256 "RTF_RGBA16f"))
  (bind _output_get (Variables|/Script/Engine.SceneCaptureComponent2D|SetTextureTarget _scenecapturecomponent2d_2 _returnvalue_2))
  (Variables|/Script/Engine.SceneCaptureComponent|SetShowOnlyActors _scenecapturecomponent2d_2 (Utilities|Array|MakeArray self))
  (bind _returnvalue_3 (Rendering|Material|CreateDynamicMaterialInstance "/Game/M_Render.M_Render" "None" "None" :!class /Script/Engine.KismetMaterialLibrary))
  (Variables|Default|SetRender _returnvalue_3)
  (Rendering|Material|SetTextureParameterValue _returnvalue_3 "Render" _output_get)
  (Utilities|FlowControl|Delay 0.5)
  (Rendering|SceneCapture|CaptureScene _scenecapturecomponent2d_2 :!class /Script/Engine.SceneCaptureComponent2D)
  (Actor|DestroyActor))

(event Collision|EventActorBeginOverlap
  (params (OtherActor :type Actor%20Object%20Reference)))

(event EventTick
  (params (DeltaSeconds :type Float%20%28single-precision%29)))

(fn ConstructionScript)